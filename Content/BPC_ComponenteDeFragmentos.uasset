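; Actor component that tracks collection of the fragments needed to complete a key (llave).
; BeginPlay stores the size of the Fragmentos array as the target, then prints needed and collected counts every second through a looping Delay.
; GetFragment removes the given item from the array, counts only successful removals and calls the LlaveCompleta dispatcher when the count reaches the target.
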(event `self.ReceiveBeginPlay`
  (set `self.FragmentosARecoger` (`KismetArrayLibrary.Array_Length` (`self.Fragmentos`)))
  (`KismetSystemLibrary.PrintString` (`KismetStringLibrary.Concat_StrStr` "Fragmentos necesarios: " (`KismetStringLibrary.Conv_IntToString` (`self.FragmentosARecoger`)) " \nFragmentos recogidos: " (`KismetStringLibrary.Conv_IntToString` (`self.Recogidos`))) true true (struct :`G` 0.66 :`B` 1.0 :`A` 1.0) 1.0 :!label _label)
  (`KismetSystemLibrary.Delay` 1.0)
  (goto _label))

(event `self.ReceiveTick`
  (params (DeltaSeconds :type "Float (single-precision)")))

(fn `GetFragment`
  (params (ItemFrag :type "/Game/Entrega1/BP_ItemFragmenteLlave Object Reference"))
  (bind _returnvalue (`KismetArrayLibrary.Array_RemoveItem` (`self.Fragmentos`) ItemFrag))
  (if _returnvalue
    (bind _output_get (set `self.Recogidos` (+ (`self.Recogidos`) 1)))
    (if (== _output_get (`self.FragmentosARecoger`))
      (`self.LlaveCompleta`))))